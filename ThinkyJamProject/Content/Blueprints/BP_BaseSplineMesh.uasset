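; Spline-mesh string that connects the pins of two pieces of evidence and follows them while flagged as moving.
; UpdateSplineMesh samples points between the endpoints, offsets their Z by StringCurve times CurveStrength, then lays mesh segments along the spline, recycling hidden components from a pool.
; Mouse movement drives CurveStrength before placement and while evidence moves; after PlaceDownString, a self-rescheduling timer eases it down to a resting value.
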(event Custom|PlaceDownString
  (params (CurveStrength :type Float%20%28double-precision%29) (EvidenceConnection :type S%20Evidence%20Connection%20Structure))
  (Variables|Default|SetCurveStrength CurveStrength)
  (bind _output_get (Variables|Default|SetEvidenceConnection EvidenceConnection))
  (Variables|Default|SetPlacedDown true)
  (CallFunction|UpdateSplineMesh (Transformation|GetWorldLocation (Variables|/Game/Blueprints/BP_Evidence.BP_Evidence_C|GetPin (.evidencea _output_get))) (Transformation|GetWorldLocation (Variables|/Game/Blueprints/BP_Evidence.BP_Evidence_C|GetPin (.evidenceb _output_get))))
  (CallFunction|CurveStringEvent))

(event Custom|CurveStringEvent
  (if (> (Variables|Default|GetCurveStrength) 5.0)
    (Variables|Default|SetCurveStrength (- (Variables|Default|GetCurveStrength) (* (Utilities|Time|GetWorldDeltaSeconds) 2.0)))
    (CallFunction|UpdateSplineMesh (Variables|Default|GetStartLoc) (Variables|Default|GetEndLoc))
    (Utilities|Time|SetTimerbyEvent (delegate Custom|CurveStringEvent) (Utilities|Time|GetWorldDeltaSeconds))))

(event EventTick
  (params (DeltaSeconds :type Float%20%28single-precision%29))
  (bind _evidenceconnection (Variables|Default|GetEvidenceConnection))
  (if (Variables|Default|GetPlacedDown)
    (if (Variables|Default|GetShouldUpdateBecauseEvidenceIsMoving)
      (CallFunction|UpdateCurveStrength)
      (CallFunction|UpdateSplineMesh (Transformation|GetWorldLocation (Variables|/Game/Blueprints/BP_Evidence.BP_Evidence_C|GetPin (.evidencea _evidenceconnection))) (Transformation|GetWorldLocation (Variables|/Game/Blueprints/BP_Evidence.BP_Evidence_C|GetPin (.evidenceb _evidenceconnection)))))
    (else
      (CallFunction|UpdateCurveStrength))))

(fn ConstructionScript)

(fn UpdateSplineMesh
  (params (Start :type Vector) (End :type Vector))
  (Utilities|Array|Clear (Variables|Default|GetPoints))
  (Variables|Default|SetStartLoc Start)
  (Variables|Default|SetEndLoc End)
  (bind _output_get (Variables|Default|SetDistance (Math|Vector|Distance(Vector) (Variables|Default|GetStartLoc) (Variables|Default|GetEndLoc))))
  (Variables|Default|SetAmountSections (Math|Float|Truncate (/ _output_get (Variables|Default|GetSectionLength))))
  (for _index (range 0 (Variables|Default|GetAmountSections))
    (Utilities|Array|Add (Variables|Default|GetPoints) (+ (* (Math|Vector|GetUnitDirection(Vector) (Variables|Default|GetStartLoc) (Variables|Default|GetEndLoc)) (* _index (Variables|Default|GetSectionLength))) (Variables|Default|GetStartLoc))))
  (bind _curvedvector (CallFunction|AddCurvetoPoints (Variables|Default|GetPoints)))
  (Variables|Default|SetPoints _curvedvector)
  (Spline|SetSplinePoints (Variables|Default|GetSpline) (Variables|Default|GetPoints) "World" true)
  (CallFunction|UnuseAllSplineComponents)
  (if (Variables|Default|GetAllowScaling)
    (Variables|Default|SetSectionLength (.z (Transformation|GetActorScale3D))))
  (for _index_2 (range 0 (- (Math|Float|Truncate (/ (Spline|GetSplineLength (Variables|Default|GetSpline)) (Variables|Default|GetSectionLength))) (select (Variables|Default|GetMustBeFullLengthMeshes) 1 0)))
    (CallFunction|AddSplineMeshComponent _index_2)))

(fn GetStartPosTangent
  (params (Index :type Integer))
  (bind _sectionlength (Variables|Default|GetSectionLength))
  (bind _spline (Variables|Default|GetSpline))
  (bind _returnvalue (* Index _sectionlength))
  (bind _returnvalue_2 (Spline|GetLocationatDistanceAlongSpline _spline _returnvalue "Local"))
  (bind (_x _y _z) (Math|Vector|BreakVector _returnvalue_2))
  (return (Math|Vector|MakeVector _x _y _z) (Math|Vector|ClampVectorSize (Spline|GetTangentatDistanceAlongSpline _spline _returnvalue "Local") 0.0 (Variables|Default|GetSectionLength))))

(fn GetEndPosTangent
  (params (Index :type Integer))
  (bind _returnvalue (+ Index 1))
  (bind _sectionlength (Variables|Default|GetSectionLength))
  (bind _spline (Variables|Default|GetSpline))
  (bind _returnvalue_2 (* _returnvalue _sectionlength))
  (bind _returnvalue_3 (Spline|GetLocationatDistanceAlongSpline _spline _returnvalue_2 "Local"))
  (return (Math|Vector|MakeVector (.x _returnvalue_3) (.y _returnvalue_3) (.z _returnvalue_3)) (Math|Vector|ClampVectorSize (Spline|GetTangentatDistanceAlongSpline _spline _returnvalue_2 "Local") 0.0 (Variables|Default|GetSectionLength))))

(fn DeleteSplineMesh
  (for _array_element (Actor|GetComponentsByClass "/Script/Engine.SplineMeshComponent")
    (Components|DestroyComponent _array_element)))

(fn AddSplineMeshComponent
  (params (index :type Integer))
  (LocalVariables|Setindex' index)
  (bind _splinemeshcomponent (CallFunction|GraborCreateSplineMeshComponent))
  (LocalVariables|SetCurrentComponent _splinemeshcomponent)
  (Transformation|SetMobility (LocalVariables|GetCurrentComponent) "Movable")
  (Components|StaticMesh|SetStaticMesh (LocalVariables|GetCurrentComponent) (Variables|Default|GetMeshForSpline))
  (Rendering|Material|SetMaterial (LocalVariables|GetCurrentComponent) 0 "/Game/MaterialLibrary/Debug_red.Debug_red")
  (SplineMesh|SetForwardAxis (LocalVariables|GetCurrentComponent) "Z" true)
  (SplineMesh|SetStartandEnd (LocalVariables|GetCurrentComponent) (.Position (CallFunction|GetStartPosTangent (LocalVariables|Getindex'))) (.Tangent (CallFunction|GetStartPosTangent (LocalVariables|Getindex'))) (.Position (CallFunction|GetEndPosTangent (LocalVariables|Getindex'))) (.Tangent (CallFunction|GetEndPosTangent (LocalVariables|Getindex'))) true :!class /Script/Engine.SplineMeshComponent)
  (Collision|SetCollisionEnabled (LocalVariables|GetCurrentComponent) (Variables|Default|GetCollisionType)))

(fn AddCurvetoPoints
  (params (Vector :type Array%20of%20Vectors))
  (LocalVariables|SetAmountSegments (Utilities|Array|Length Vector))
  (for (_array_element _array_index) Vector
    (Utilities|Array|Add (LocalVariables|GetCurved) (Math|Vector|MakeVector (.x _array_element) (.y _array_element) (+ (* (Variables|Default|GetCurveStrength) (Math|Curves|GetFloatValue (Variables|Default|GetStringCurve) (/ _array_index (- (LocalVariables|GetAmountSegments) 1)))) (.z _array_element)))))
  (return (LocalVariables|GetCurved)))

(fn GraborCreateSplineMeshComponent
  (if (Utilities|Array|IsValidIndex (Variables|Default|GetUnusedSplineMeshComponent))
    (Variables|Default|SetRecycledSplineMesh (Utilities|Array|Get(acopy) (Variables|Default|GetUnusedSplineMeshComponent)))
    (Utilities|Array|RemoveIndex (Variables|Default|GetUnusedSplineMeshComponent))
    (Utilities|Array|Add (Variables|Default|GetUsedSplineMeshComponents) (Variables|Default|GetRecycledSplineMesh))
    (Rendering|SetVisibility (Variables|Default|GetRecycledSplineMesh) true false)
    (return (Variables|Default|GetRecycledSplineMesh))
    (else
      (bind _returnvalue (AddComponent|AddSplineMeshComponent true))
      (Utilities|Array|Add (Variables|Default|GetUsedSplineMeshComponents) _returnvalue)
      (return _returnvalue))))

(fn UnuseAllSplineComponents
  (for _array_element (Variables|Default|GetUsedSplineMeshComponents)
    (Rendering|SetVisibility _array_element false false)
    (Utilities|Array|Add (Variables|Default|GetUnusedSplineMeshComponent) _array_element))
  (Utilities|Array|Clear (Variables|Default|GetUsedSplineMeshComponents)))

(fn UpdateCurveStrength
  (bind _tj_player_controller (CallFunction|GetTJPlayerController))
  (bind (_deltax _deltay) (Class|PlayerController|GetInputMouseDelta _tj_player_controller))
  (bind _returnvalue (Math|Vector2D|Vector2DLength (Math|Vector2D|MakeVector2D _deltax _deltay)))
  (if (< _returnvalue (Variables|Default|GetCursorMovement))
    (Variables|Default|SetCursorMovement (- (Variables|Default|GetCursorMovement) (* (Utilities|Time|GetWorldDeltaSeconds) 15.0)))
    (else
      (Variables|Default|SetCursorMovement _returnvalue)))
  (Variables|Default|SetCurveStrength (Math|Interpolation|FInterpTo (Variables|Default|GetCurveStrength) (Math|Float|Min(Float) (+ (Math|Float|MakeLiteralFloat 5.0) (* (Variables|Default|GetCursorMovement) 5e+01)) 5e+01) 8.0 (Utilities|Time|GetWorldDeltaSeconds))))