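; Evidence item on an investigation board that the player drags around and links to other evidence with strings.
; Clicking the plane makes it follow a cursor trace across boards, switching to that board's camera and flagging connected strings to update.
; Dragging from the pin previews a string; releasing on another pin connects both through BPEvidenceConnections.
; InitializeBaseEvidence scales the plane and textures it with a render target of its widget class.
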(event Custom|OnClickEvidence
  (bind _tj_player_controller (CallFunction|GetTJPlayerController))
  ;[1 1 1] Evidence
  (Variables|/Game/Core/TJ_PlayerController.TJ_PlayerController_C|SetDraggedEvidence _tj_player_controller self)
  (Variables|/Game/Core/TJ_PlayerController.TJ_PlayerController_C|SetDraggingEvidence _tj_player_controller true)
  (Variables|Default|SetIsEvidenceBeingDragged true))

(event Custom|OnReleaseEvidence
  (bind _tj_player_controller (CallFunction|GetTJPlayerController))
  ;[1 1 1] Evidence
  (Variables|/Game/Core/TJ_PlayerController.TJ_PlayerController_C|SetDraggedEvidence _tj_player_controller 0)
  (Variables|/Game/Core/TJ_PlayerController.TJ_PlayerController_C|SetDraggingEvidence _tj_player_controller false)
  (Variables|Default|SetIsEvidenceBeingDragged false)
  (Default|MakeAllStringsStopMoving (Variables|/Game/Core/TJ_GameMode.TJ_GameMode_C|GetBP_EvidenceConnections (CallFunction|GetTJGameMode))))

(event Custom|PinOC
  (params (TouchedComponent :type Primitive%20Component%20Object%20Reference) (ButtonPressed :type Key%20Structure :default "None"))
  (CallFunction|OnClickPin))

(event Custom|PinOR
  (params (TouchedComponent :type Primitive%20Component%20Object%20Reference) (ButtonReleased :type Key%20Structure :default "None"))
  (CallFunction|OnReleasePin))

(event Custom|OnHoverEvidence
  ;[1 1 1] Evidence
  (CallFunction|ShowTooltipOverActor self "Drag to move"))

(event Custom|OnClickPin
  (bind _tj_player_controller (CallFunction|GetTJPlayerController))
  (Variables|/Game/Core/TJ_PlayerController.TJ_PlayerController_C|SetDraggedEvidence _tj_player_controller self)
  (Variables|Default|SetIsStringBeingDragged true)
  (Variables|/Game/Core/TJ_PlayerController.TJ_PlayerController_C|SetDraggingString _tj_player_controller true))

(event Custom|OnReleasePin
  (bind _tj_player_controller (CallFunction|GetTJPlayerController))
  (if (Variables|/Game/Core/TJ_PlayerController.TJ_PlayerController_C|GetDraggingString _tj_player_controller)
    (if (not (== (Variables|/Game/Core/TJ_PlayerController.TJ_PlayerController_C|GetDraggedEvidence _tj_player_controller) self))
      (Default|ConnectEvidences (Variables|/Game/Core/TJ_GameMode.TJ_GameMode_C|GetBP_EvidenceConnections (CallFunction|GetTJGameMode)) (Variables|/Game/Core/TJ_PlayerController.TJ_PlayerController_C|GetDraggedEvidence (CallFunction|GetTJPlayerController)) self))))

(event Custom|OnHoverPin
  (bind _tj_player_controller (CallFunction|GetTJPlayerController))
  (if (Variables|/Game/Core/TJ_PlayerController.TJ_PlayerController_C|GetDraggingString _tj_player_controller)
    (if (not (== (Variables|/Game/Core/TJ_PlayerController.TJ_PlayerController_C|GetDraggedEvidence _tj_player_controller) self))
      (CallFunction|ShowTooltipOverActor self "Release to connect to this evidence"))
    (else
      (CallFunction|ShowTooltipOverActor self "Drag string connection from this pin"))))

(event Custom|PlaneBCO
  (params (TouchedComponent :type Primitive%20Component%20Object%20Reference))
  (CallFunction|OnHoverEvidence))

(event Custom|PlaneOC
  (params (TouchedComponent :type Primitive%20Component%20Object%20Reference) (ButtonPressed :type Key%20Structure :default "None"))
  (CallFunction|OnClickEvidence))

(event Custom|PlaneOR
  (params (TouchedComponent :type Primitive%20Component%20Object%20Reference) (ButtonReleased :type Key%20Structure :default "None"))
  (CallFunction|OnReleaseEvidence))

(event Custom|PinBCO
  (params (TouchedComponent :type Primitive%20Component%20Object%20Reference))
  (CallFunction|OnHoverPin))

(event EventBeginPlay
  (bind _plane (Variables|Default|GetPlane))
  (bind _pin (Variables|Default|GetPin))
  (Variables|Default|SetBoard (Components|GetOwner))
  (EventDispatchers|BindEventtoOnBeginCursorOver _plane (delegate Custom|PlaneBCO))
  (EventDispatchers|BindEventtoOnClicked _plane (delegate Custom|PlaneOC))
  (EventDispatchers|BindEventtoOnReleased _plane (delegate Custom|PlaneOR))
  (EventDispatchers|BindEventtoOnBeginCursorOver _pin (delegate Custom|PinBCO))
  (EventDispatchers|BindEventtoOnClicked _pin (delegate Custom|PinOC))
  (EventDispatchers|BindEventtoOnReleased _pin (delegate Custom|PinOR)))

(event Collision|EventActorBeginOverlap
  (params (OtherActor :type Actor%20Object%20Reference)))

(event EventTick
  (params (DeltaSeconds :type Float%20%28single-precision%29))
  (Variables|Default|SetHitResultBoard (.HitResult (Game|Player|GetHitResultUnderCursorbyChannel (CallFunction|GetTJPlayerController) "TraceTypeQuery3" true)))
  (CallFunction|DragEvidenceOverBoard)
  (CallFunction|DragStringfromPin))

(fn ConstructionScript)

(fn DragEvidenceOverBoard
  (bind _hitresultboard (Variables|Default|GetHitResultBoard))
  (bind (_bblockinghit _binitialoverlap _time _distance _location _impactpoint _normal _impactnormal _physmat _hitactor) (Collision|BreakHitResult _hitresultboard))
  (Variables|Default|SetCursorOnBoardLocation _location)
  (if (Variables|Default|GetIsEvidenceBeingDragged)
    (if _bblockinghit
      (Transformation|SetActorLocation (Math|Interpolation|VInterpTo (Transformation|GetActorLocation) (+ _location (* _normal 2.0)) (Utilities|Time|GetWorldDeltaSeconds) 12.0) false false)
      (Transformation|SetActorRotation (Transformation|GetActorRotation _hitactor))
      (CallFunction|UpdateStringsonEvidenceMove)
      (bind _asbp_board_base (Utilities|Casting|CastToBP_BoardBase _hitactor))
      (if (Utilities|Enum|NotEqual(Enum) (Variables|/Game/Blueprints/BP_BoardBase.BP_BoardBase_C|GetAttachedCameraPosition _asbp_board_base) (Variables|/Game/Core/TJ_PlayerController.TJ_PlayerController_C|GetCurrentCameraPosition (CallFunction|GetTJPlayerController)))
        (Default|SetCameraPosition (CallFunction|GetTJPlayerController) (Variables|/Game/Blueprints/BP_BoardBase.BP_BoardBase_C|GetAttachedCameraPosition _asbp_board_base))))))

(fn DragStringfromPin
  (bind _cursoronboardlocation (Variables|Default|GetCursorOnBoardLocation))
  (if (Variables|Default|GetIsStringBeingDragged)
    (if (Utilities|Operators|NotEqual(!=) _cursoronboardlocation (Math|Vector|VectorZero) 0.01)
      (Default|SetUnconnectedSplinePoints (Variables|/Game/Core/TJ_GameMode.TJ_GameMode_C|GetBP_EvidenceConnections (CallFunction|GetTJGameMode)) (Transformation|GetWorldLocation (Variables|Default|GetPin)) _cursoronboardlocation)
      (else
        (Default|SetUnconnectedSplinePoints (Variables|/Game/Core/TJ_GameMode.TJ_GameMode_C|GetBP_EvidenceConnections (CallFunction|GetTJGameMode)) "0, 0, 0" "0, 0, 0")))))

(fn UpdateStringsonEvidenceMove
  (for _array_element (Default|GetAllConnectedSplinesOfEvidence (Variables|/Game/Core/TJ_GameMode.TJ_GameMode_C|GetBP_EvidenceConnections (CallFunction|GetTJGameMode)) self)
    (Variables|/Game/Blueprints/BP_BaseSplineMesh.BP_BaseSplineMesh_C|SetShouldUpdateBecauseEvidenceIsMoving _array_element true)))

(fn ScalePlanetoWidget
  (bind _bpwidgetreference (Variables|Default|GetBPWidgetReference))
  (bind _setting_scalefactor (Variables|Default|GetSetting_ScaleFactor))
  (bind _manuallysetdesiredsize (Utilities|GetClassDefaults _bpwidgetreference))
  (bind _returnvalue (* _manuallysetdesiredsize _setting_scalefactor))
  (Transformation|SetWorldScale3D (Variables|Default|GetPlane) (Math|Vector|MakeVector (.x _returnvalue) (.y _returnvalue) 1.0)))

(fn SetPlaneMaterialtoWidgetTexture
  (bind _returnvalue (Rendering|Material|CreateDynamicMaterialInstance "/Game/UI/EvidenceWidgets/RenderTargets/M_EvidenceMat.M_EvidenceMat" "None" "None" :!class /Script/Engine.KismetMaterialLibrary))
  (Variables|Default|SetDynamicMaterial _returnvalue)
  (Rendering|Material|SetMaterial (Variables|Default|GetPlane) 0 (Variables|Default|GetDynamicMaterial))
  (bind _rendertarget (Default|GetRenderTargetforWidgetClass (Variables|/Game/Core/TJ_GameMode.TJ_GameMode_C|GetBP_EvidenceRenderTextureCreator (CallFunction|GetTJGameMode)) (Variables|Default|GetBPWidgetReference)))
  (Rendering|Material|SetTextureParameterValue (Variables|Default|GetDynamicMaterial) "RenderTexture" _rendertarget))

(fn InitializeBaseEvidence
  (CallFunction|ScalePlanetoWidget)
  (CallFunction|SetPlaneMaterialtoWidgetTexture))