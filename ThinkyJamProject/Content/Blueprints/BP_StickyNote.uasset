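; BP_StickyNote is a clickable sticky note actor with an editable text widget.
; On BeginPlay it takes a unique ID from an incrementing counter on TJ_GameMode and registers itself as the Owner of its WBP_TextInput.
; A simple double-click detector counts clicks and focuses the text box from the second one, resetting the count after a short delay following mouse release.
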(event EventBeginPlay
  (|CallParentFunction)
  (bind _astj_game_mode (Utilities|Casting|CastToTJ_GameMode (Game|GetGameMode))
    (:then
      (Variables|Default|SetID (Variables|/Game/Core/TJ_GameMode.TJ_GameMode_C|GetStickyNoteStartID _astj_game_mode))
      (Variables|/Game/Core/TJ_GameMode.TJ_GameMode_C|SetStickyNoteStartID _astj_game_mode (+ (Variables|/Game/Core/TJ_GameMode.TJ_GameMode_C|GetStickyNoteStartID _astj_game_mode) 1)))
    (:CastFailed
      _))
  (bind _aswbp_text_input (Utilities|Casting|CastToWBP_TextInput (UserInterface|GetWidget (Variables|Default|GetTextWidget))))
  (Variables|/Game/UI/Widgets/WBP_TextInput.WBP_TextInput_C|SetOwner _aswbp_text_input self))

(event Collision|EventActorBeginOverlap
  (params (OtherActor :type Actor%20Object%20Reference))
  (|CallParentFunction OtherActor) ; This node is disabled and will not be called.\nDrag off pins to build functionality.
)

(event EventTick
  (params (DeltaSeconds :type Float%20%28single-precision%29))
  (|CallParentFunction DeltaSeconds) ; This node is disabled and will not be called.\nDrag off pins to build functionality.
)

(event EventActorOnClicked
  (params (ButtonPressed :type Key%20Structure))
  (|CallParentFunction ButtonPressed)
  (Variables|Default|SetClickCount (+ (Variables|Default|GetClickCount) 1)) ; This is stupid but hey, it works
  (if (>= (Variables|Default|GetClickCount) 2)
    (bind _aswbp_text_input (Utilities|Casting|CastToWBP_TextInput (UserInterface|GetWidget (Variables|Default|GetTextWidget))))
    (Widget|SetFocus (Variables|/Game/UI/Widgets/WBP_TextInput.WBP_TextInput_C|GetTextBox _aswbp_text_input))))

(event EventActorOnReleased
  (params (ButtonReleased :type Key%20Structure))
  (|CallParentFunction ButtonReleased)
  (Utilities|FlowControl|Delay 1.0)
  (Variables|Default|SetClickCount 0))

(fn ConstructionScript
  (|CallParentFunction))