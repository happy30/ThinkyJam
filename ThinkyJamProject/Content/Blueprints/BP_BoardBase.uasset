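; BP_BoardBase is a base actor for clickable boards that move the player's camera to an attached camera position.
; On click, it passes that position to the TJ player controller's SetCameraPosition and hides the tooltip.
; On cursor hover, it shows its tooltip text over the actor, unless the camera is already at that position.
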(event EventBeginPlay)

(event Collision|EventActorBeginOverlap
  (params (OtherActor :type Actor%20Object%20Reference)))

(event EventTick
  (params (DeltaSeconds :type Float%20%28single-precision%29)))

(event MouseInput|EventActorOnClicked
  (params (ButtonPressed :type Key%20Structure :default "None"))
  (Default|SetCameraPosition (CallFunction|GetTJPlayerController) (Variables|Default|GetAttachedCameraPosition))
  (CallFunction|HideTooltip))

(event MouseInput|EventActorBeginCursorOver
  (if (Utilities|Enum|NotEqual(Enum) (Variables|/Game/Core/TJ_PlayerController.TJ_PlayerController_C|GetCurrentCameraPosition (CallFunction|GetTJPlayerController)) (Variables|Default|GetAttachedCameraPosition))
    (CallFunction|ShowTooltipOverActor self (Variables|Default|GetTooltipText))))

(fn ConstructionScript)