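; Player pawn that views the game through placed camera position actors, blending the player controller's view target between them.
; BeginPlay caches each camera's FOV and rotation, then moves to an initial position.
; Tick eases the active camera's FOV toward a target that StartZoom and EndZoom switch between zoomed and cached values.
; AddCameraSway eases the camera's pitch and yaw around its cached rotation, with stronger sway while zoomed in.
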(event EventBeginPlay
  (for _array_element (Variables|Default|GetCameraPositions)
    (Utilities|Array|Add (Variables|Default|GetTargetFOVNormal) (Variables|/Script/Engine.CameraComponent|GetFieldOfView (Variables|/Script/Engine.CameraActor|GetCameraComponent _array_element))))
  (for _array_element_2 (Variables|Default|GetCameraPositions)
    (Utilities|Array|Add (Variables|Default|GetDefaultRotators) (Transformation|GetActorRotation _array_element_2)))
  (CallFunction|LerptoCameraPosition "NewEnumerator0"))

(event EventTick
  (params (DeltaSeconds :type Float%20%28single-precision%29))
  (bind _currentcamerapos (Variables|Default|GetCurrentCameraPos))
  (bind _cameracomponent (Variables|/Script/Engine.CameraActor|GetCameraComponent _currentcamerapos))
  (Camera|SetFieldOfView _cameracomponent (Math|Interpolation|FInterpTo (Variables|/Script/Engine.CameraComponent|GetFieldOfView _cameracomponent) (Variables|Default|GetTargetFOV) (Utilities|Time|GetWorldDeltaSeconds) 8.0)))

(fn ConstructionScript)

(fn LerptoCameraPosition
  (params (CameraPosition :type E_CameraPosition%20Enum :default "NewEnumerator0"))
  (bind _array_element (Utilities|Array|ForEachLoopwithBreak (Variables|Default|GetCameraPositions) :!label _label)
    (:LoopBody
      (if (Utilities|Enum|Equal(Enum) CameraPosition (Variables|/Game/Core/BP_CameraPosition.BP_CameraPosition_C|GetCameraPos _array_element))
        (Variables|Default|SetCurrentCameraPos _array_element)
        (goto _label Break)))
    (:Completed
      (Game|Player|SetViewTargetwithBlend (CallFunction|GetTJPlayerController) (Variables|Default|GetCurrentCameraPos) 0.6 "VTBlend_EaseInOut" 2.0 false)
      (Variables|Default|SetTargetFOV (Utilities|Array|Get(acopy) (Variables|Default|GetTargetFOVNormal) (CallFunction|GetCurrentCameraIndex))))))

(fn AddCameraSway
  (params (SwayAmount :type Vector%202D%20Structure))
  (bind _camerapositions (Variables|Default|GetCameraPositions))
  (bind _currentcamerapos (Variables|Default|GetCurrentCameraPos))
  (bind _defaultrotators (Variables|Default|GetDefaultRotators))
  (bind _zoomedin (Variables|Default|GetZoomedIn))
  (bind _returnvalue (Utilities|Array|FindItem _camerapositions _currentcamerapos))
  (bind _returnvalue_2 (Math|Float|SelectFloat 3.0 1.0 _zoomedin))
  (bind _output (Utilities|Array|Get(acopy) _defaultrotators _returnvalue))
  (bind _returnvalue_3 (* SwayAmount _returnvalue_2))
  (bind (_x _y) (Math|Vector2D|BreakVector2D _returnvalue_3))
  (Transformation|SetActorRotation (Variables|Default|GetCurrentCameraPos) (Math|Interpolation|RInterpTo (Transformation|GetActorRotation (Variables|Default|GetCurrentCameraPos)) (Math|Rotator|MakeRotator 0.0 (+ (.pitch _output) (* _y -1.0)) (+ (.yaw _output) _x)) (Utilities|Time|GetWorldDeltaSeconds) 8.0)))

(fn StartZoom
  (Variables|Default|SetTargetFOV (Variables|Default|GetTargetFOVZoomedIn))
  (Variables|Default|SetZoomedIn true))

(fn EndZoom
  (Variables|Default|SetTargetFOV (Utilities|Array|Get(acopy) (Variables|Default|GetTargetFOVNormal) (CallFunction|GetCurrentCameraIndex)))
  (Variables|Default|SetZoomedIn false))

(fn GetCurrentCameraIndex
  (return (Utilities|Array|FindItem (Variables|Default|GetCameraPositions) (Variables|Default|GetCurrentCameraPos))))