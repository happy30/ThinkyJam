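; BP_EvidenceRenderTextureCreator pre-renders evidence widgets into render targets when play begins.
; BeginPlay creates each class in EvidenceWidgets and draws it with nearest filtering to the same-index entry in RenderTargets, sized from that class's defaults.
; Once all are drawn, it calls InitializeBaseEvidence on every BP_Evidence actor in the world.
; GetRenderTargetForWidgetClass uses the parallel arrays to return the render target matching a widget class.
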(event EventBeginPlay
  (for (_array_element _array_index) (Variables|Default|GetEvidenceWidgets)
    (bind _returnvalue (UserInterface|CreateWidget _array_element))
    (Class|RenderWidgettoTargetPluginBPLibrary|DrawWidgettoTarget (Utilities|Array|Get(acopy) (Variables|Default|GetRenderTargets) _array_index) _returnvalue (Utilities|GetClassDefaults _array_element) false "TF_Nearest" 0.0))
  (bind _outactors (Actor|GetAllActorsOfClass "/Game/Blueprints/BP_Evidence.BP_Evidence_C"))
  (for _array_element_2 _outactors
    (Default|InitializeBaseEvidence _array_element_2)))

(event EventTick
  (params (DeltaSeconds :type Float%20%28single-precision%29)))

(fn GetRenderTargetforWidgetClass
  (params (WidgetClass :type WBP%20Evidence%20Base%20Widget%20Class%20Reference))
  (return (Utilities|Array|Get(acopy) (Variables|Default|GetRenderTargets) (Utilities|Array|FindItem (Variables|Default|GetEvidenceWidgets) WidgetClass))))